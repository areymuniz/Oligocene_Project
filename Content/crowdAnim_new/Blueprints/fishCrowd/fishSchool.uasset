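; Fish school spawner that populates a crowd of AI-controlled fish and hands them to a worker engine.
; On BeginPlay it samples points in a rotated ellipsoidal shell, with bounded retries against overlaps, then spawns and configures fish pawns with controllers.
; One spawned FishEngine receives the fish, positions, alive flags and target net data, and becomes each fish's worker.
; Tick destroys that engine once it is dead and clears the lists.
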(event `self.ReceiveBeginPlay`
  (for _index (range (`self.fishNumber`))
    (bind (_fish _outputvec) (`self.Add Fish` _index))
    (`KismetArrayLibrary.Array_AddUnique` (`self.fishArray`) _fish)
    (`KismetArrayLibrary.Array_AddUnique` (`self.fishLocArray`) _outputvec)
    (`KismetArrayLibrary.Array_Add` (`self.aliveArray`) true))
  (bind _returnvalue (`|SpawnActorFromClass` "/Game/crowdAnim_new/Blueprints/fishCrowd/fishEngine.fishEngine_C" (`KismetMathLibrary.MakeTransform` (0.0 0.0 0.0)) "Undefined" "OverrideRootScale" null null))
  (`KismetArrayLibrary.Array_AddUnique` (`self.currentEngine`) _returnvalue)
  (set `/Game/crowdAnim_new/Blueprints/fishCrowd/fishEngine.aliveArray` (`self.aliveArray`) _returnvalue)
  (bind _output_get (set `/Game/crowdAnim_new/Blueprints/fishCrowd/fishEngine.workerFishLIst` (`self.fishArray`) _returnvalue))
  (set `/Game/crowdAnim_new/Blueprints/fishCrowd/fishEngine.fishTargetArray` (`self.fishLocArray`) _returnvalue)
  (set `/Game/crowdAnim_new/Blueprints/fishCrowd/fishEngine.fishNetLocation` (`self.K2_GetActorLocation` (`self.targetFishNet`)) _returnvalue)
  (set `/Game/crowdAnim_new/Blueprints/fishCrowd/fishEngine.workerNetRadius` (`self.fishNetRadius`) _returnvalue)
  (for _array_element _output_get
    (set `/Game/crowdAnim_new/Blueprints/fishCrowd/BP_fishPawn.assignedWorker` _returnvalue _array_element)))

(event `self.ReceiveTick`
  (params (DeltaSeconds :type "Float (single-precision)"))
  (bind _output (`|GetArrayItem` (`self.currentEngine`)))
  (if (== (`KismetArrayLibrary.Array_Length` (`self.currentEngine`)) 1)
    (if (`/Game/crowdAnim_new/Blueprints/fishCrowd/fishEngine.dead` _output)
      (`self.K2_DestroyActor` _output)
      (`KismetArrayLibrary.Array_Clear` (`self.fishArray`))
      (`KismetArrayLibrary.Array_Clear` (`self.currentEngine`)))))

(fn `Add Fish`
  (params (fshIndex :type Integer))
  (returns (fish :type "/Game/crowdAnim_new/Blueprints/fishCrowd/BP_fishPawn Object Reference") (outputVec :type "Vector Structure"))
  (locals (overLapStatus :type Boolean :default true) (generatedLoc :type "Vector Structure") (loopNum :type Integer))
  (bind _returnvalue (`self.K2_GetActorLocation`))
  (while (and (`local.overLapStatus`) (<= (`local.loopNum`) (`self.loopmax`)))
    (bind _newparam (`self.generateEllipsoid` (`self.spawnScale`) (`self.spawnRadius`) _returnvalue (`self.innerRadius`) (`self.K2_GetActorRotation`)))
    (bind _output (`self.checkOverlapWithOthers` _newparam))
    (set `local.overLapStatus` _output)
    (set `local.generatedLoc` _newparam)
    (set `local.loopNum` (+ (`local.loopNum`) 1)))
  (set `local.loopNum` 0)
  (bind _returnvalue_2 (`|SpawnActorFromClass` (`self.fishMesh`) (`KismetMathLibrary.MakeTransform` (`local.generatedLoc`)) "AlwaysSpawn" "OverrideRootScale" null null))
  (set `/Game/crowdAnim_new/Blueprints/fishCrowd/BP_fishPawn.startingOrigLoc` _returnvalue _returnvalue_2)
  (set `/Game/crowdAnim_new/Blueprints/fishCrowd/BP_fishPawn.fishIndex` fshIndex _returnvalue_2)
  (set `/Game/crowdAnim_new/Blueprints/fishCrowd/BP_fishPawn.speedArray` (`self.speedArray`) _returnvalue_2)
  (set `/Game/crowdAnim_new/Blueprints/fishCrowd/BP_fishPawn.shapeList` (`self.shapeList`) _returnvalue_2)
  (set `/Game/crowdAnim_new/Blueprints/fishCrowd/BP_fishPawn.birthLoc` (- (`local.generatedLoc`) (`self.K2_GetActorLocation`)) _returnvalue_2)
  (set `/Game/crowdAnim_new/Blueprints/fishCrowd/BP_fishPawn.schoolParent` self _returnvalue_2)
  (set `Pawn.AIControllerClass` "/Game/crowdAnim_new/Blueprints/fishCrowd/fishController.fishController_C" _returnvalue_2)
  (`Pawn.SpawnDefaultController` _returnvalue_2)
  (`self.applyFishSettings` _returnvalue_2)
  (`self.applySchoolSettings` _returnvalue_2)
  (`self.applyMovementSettings` _returnvalue_2)
  (return _returnvalue_2 (`local.generatedLoc`)))

(fn `applyFishSettings`
  (params (fish :type "/Game/crowdAnim_new/Blueprints/fishCrowd/BP_fishPawn Object Reference"))
  (set `/Game/crowdAnim_new/Blueprints/fishCrowd/BP_fishPawn.maxFlapSpeed` (`self.maxFlapSpeed`) fish)
  (set `/Game/crowdAnim_new/Blueprints/fishCrowd/BP_fishPawn.minFlapSpeed` (`self.minFlapSpeed`) fish)
  (set `/Game/crowdAnim_new/Blueprints/fishCrowd/BP_fishPawn.maxOffset` (`self.maxColorOffset`) fish)
  (set `/Game/crowdAnim_new/Blueprints/fishCrowd/BP_fishPawn.minOffset` (`self.minColorOffset`) fish)
  (set `/Game/crowdAnim_new/Blueprints/fishCrowd/BP_fishPawn.maxGrayScaleOffset` (`self.maxGrayScaleOffset`) fish)
  (set `/Game/crowdAnim_new/Blueprints/fishCrowd/BP_fishPawn.maxScale` (`self.maxScale`) fish)
  (set `/Game/crowdAnim_new/Blueprints/fishCrowd/BP_fishPawn.minScale` (`self.minScale`) fish)
  (set `/Game/crowdAnim_new/Blueprints/fishCrowd/BP_fishPawn.meshRotation` (`self.fishRotation`) fish)
  (set `/Game/crowdAnim_new/Blueprints/fishCrowd/BP_fishPawn.speedVariation` (`self.fishSpeedVariation`) fish)
  (`/Game/crowdAnim_new/Blueprints/fishCrowd/BP_fishPawn.Assign Mesh` fish "/Game/crowdAnim_new/Blueprints/fishCrowd/sardine.sardine")
  (`/Game/crowdAnim_new/Blueprints/fishCrowd/BP_fishPawn.setMeshScale` fish)
  (`/Game/crowdAnim_new/Blueprints/fishCrowd/BP_fishPawn.Set Mesh Rotation` fish))

(fn `applyMovementSettings`
  (params (fishPawn :type "/Game/crowdAnim_new/Blueprints/fishCrowd/BP_fishPawn Object Reference"))
  (set `/Game/crowdAnim_new/Blueprints/fishCrowd/BP_fishPawn.acceptingRadius` (`self.acceptingRadius`) fishPawn)
  (set `/Game/crowdAnim_new/Blueprints/fishCrowd/BP_fishPawn.baitList` (`self.baitList`) fishPawn))

(fn `applySchoolSettings`
  (params (fish :type "/Game/crowdAnim_new/Blueprints/fishCrowd/BP_fishPawn Object Reference"))
  (set `/Game/crowdAnim_new/Blueprints/fishCrowd/BP_fishPawn.desiredDistance` (`self.desiredDistance`) fish))

(fn `Check Overlap`
  (params (locA :type "Vector Structure") (locB :type "Vector Structure"))
  (returns (output :type Boolean))
  (return (not (or (>= (`KismetMathLibrary.Abs` (- locA_X locB_X)) 6.0) (>= (`KismetMathLibrary.Abs` (- locA_Y locB_Y)) 6.0) (>= (`KismetMathLibrary.Abs` (- locA_Z locB_Z)) 10.0)))))

(fn `checkOverlapWithOthers`
  (params (inputLoc :type "Vector Structure"))
  (returns (output :type Boolean))
  (for _array_element (`self.fishLocArray`)
    (bind _output (`self.Check Overlap` _array_element inputLoc))
    (if _output
      (return true)))
  (return false))

(fn `generateEllipsoid`
  (params (ellpsoidScale :type "Vector Structure") (radius :type "Float (double-precision)") (center :type "Vector Structure") (innerRadius :type "Float (double-precision)") (inputRotation :type "Rotator Structure"))
  (returns (NewParam :type "Vector Structure"))
  (bind _returnvalue (`KismetMathLibrary.GetPI`))
  (bind _returnvalue_2 (`KismetMathLibrary.RandomFloatInRange` 0.0 _returnvalue))
  (bind _returnvalue_3 (`KismetMathLibrary.RandomFloatInRange` (* radius innerRadius) radius))
  (bind _returnvalue_4 (`KismetMathLibrary.RandomFloatInRange` 0.0 (* _returnvalue 2.0)))
  (bind _returnvalue_5 (`KismetMathLibrary.Sin` _returnvalue_2))
  (return (+ center (`KismetMathLibrary.GreaterGreater_VectorRotator` (* ellpsoidScale (`KismetMathLibrary.MakeVector` (* _returnvalue_5 (`KismetMathLibrary.Cos` _returnvalue_4) _returnvalue_3) (* _returnvalue_3 _returnvalue_5 (`KismetMathLibrary.Sin` _returnvalue_4)) (* (`KismetMathLibrary.Cos` _returnvalue_2) _returnvalue_3))) inputRotation))))

(fn `UserConstructionScript`)