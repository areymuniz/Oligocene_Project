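; Fish pawn for a crowd simulation that swims through a looping list of baits via floating pawn movement, turning toward its steering direction each tick.
; At each bait it picks a random offset inside the next ellipsoid shape, retrying against the assigned worker's shared targets to limit overlap.
; Flocking separation, cohesion and alignment are disconnected, leaving bait seeking as the active behavior.
; Helper functions randomize mesh scale and material color and flap animation.
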(event `self.ReceiveTick`
  (params (DeltaSeconds :type "Float (single-precision)"))
  (`self.K2_SetActorRotation` (`KismetMathLibrary.RLerp` (`self.K2_GetActorRotation`) (`self.rotation`) (* DeltaSeconds (`self.turnSpeed`))))
  (`self.applyBehaviors`))

(event `self.ReceiveBeginPlay`
  (bind (_output_x _output_y _output_z _output_w) (`KismetMathLibrary.BreakVector4` (`|GetArrayItem` (`self.shapeList`) (`self.shapeIndex`))))
  (bind _asfloating_pawn_movement (cast `FloatingPawnMovement` (`self.MovementComponent`)))
  (set `FloatingPawnMovement.MaxSpeed` (`self.Speed`) _asfloating_pawn_movement)
  (set `FloatingPawnMovement.TurningBoost` (`self.turnSpeed`) _asfloating_pawn_movement)
  (set `MovementComponent.Velocity` (5.0 5.0 5.0) _asfloating_pawn_movement)
  (`KismetSystemLibrary.Delay` 0.1)
  (if (== _output_w -1.0)
    (set `self.addOn_global` (`self.birthLoc`))
    (else
      (bind _output (`self.Generate Ellipsoid` (`KismetMathLibrary.MakeVector` _output_x _output_y _output_z) _output_w (0.0 0.0 0.0) (`self.K2_GetActorRotation` (`|GetArrayItem` (`self.baitList`) (`self.baitIndex`)))))
      (set `self.addOn_global` _output))))

(fn `applyBehaviors`
  (bind _steer (`self.swimToBaits`))
  (set `self.swimToForce` _steer)
  (`self.applyForces`))

(fn `applyForce`
  (params (force :type "Vector Structure"))
  (bind _force (`local.force`))
  (if (not (`KismetMathLibrary.Vector_IsNAN` force))
    (bind _output_get (set `self.steering` (+ (`self.GetVelocity`) _force)))
    (`PawnMovementComponent.AddInputVector` (`self.MovementComponent`) _force false)
    (set `self.rotation` (`KismetMathLibrary.Conv_VectorToRotator` _output_get))))

(fn `applyForces`
  (bind _output_get (set `self.finalForce` (+ (`self.swimToForce`) (`self.seperationForce`) (* (`self.cohesionForce`) 0) (`self.alignmentForce`))))
  (`self.applyForce` _output_get))

(fn `Assign Mesh`
  (params (fishMesh :type "StaticMesh Object Reference"))
  (bind _meshcomponent (`self.MeshComponent`))
  (`StaticMeshComponent.SetStaticMesh` _meshcomponent fishMesh)
  (bind _returnvalue (`PrimitiveComponent.CreateDynamicMaterialInstance` _meshcomponent 0 (`self.masterMat`) "None"))
  (`self.AssignMaterial` _returnvalue)
  (`PrimitiveComponent.SetMaterial` _meshcomponent 0 _returnvalue))

(fn `AssignMaterial`
  (params (inputMat :type "MaterialInstanceDynamic Object Reference"))
  (bind _maxgrayscaleoffset (`self.maxGrayScaleOffset`))
  (bind _maxoffset (`self.maxOffset`))
  (bind _minoffset (`self.minOffset`))
  (`MaterialInstanceDynamic.SetVectorParameterValue` inputMat "colorOffset" (make `LinearColor` (`KismetMathLibrary.RandomFloatInRange` _minoffset _maxoffset) (`KismetMathLibrary.RandomFloatInRange` _minoffset _maxoffset) (`KismetMathLibrary.RandomFloatInRange` _minoffset _maxoffset) 1.0))
  (`MaterialInstanceDynamic.SetScalarParameterValue` inputMat "FlapSpeed" (`KismetMathLibrary.RandomFloatInRange` (`self.minFlapSpeed`) (`self.maxFlapSpeed`)))
  (`MaterialInstanceDynamic.SetScalarParameterValue` inputMat "cycleDelay" (`KismetMathLibrary.RandomFloatInRange` -4.0 4.0))
  (`MaterialInstanceDynamic.SetScalarParameterValue` inputMat "grayScaleOffset" (`KismetMathLibrary.RandomFloatInRange` (* _maxgrayscaleoffset -1.0) _maxgrayscaleoffset)))

(fn `Check Overlap`
  (params (locA :type "Vector Structure") (locB :type "Vector Structure"))
  (returns (output :type Boolean))
  (return (not (or (>= (`KismetMathLibrary.Abs` (- locA_X locB_X)) 6.0) (>= (`KismetMathLibrary.Abs` (- locA_Y locB_Y)) 6.0) (>= (`KismetMathLibrary.Abs` (- locA_Z locB_Z)) 10.0)))))

(fn `checkOverlapWithOthers`
  (params (inputVec :type "Vector Structure"))
  (returns (output :type Boolean))
  (for (_array_element _array_index) (`/Game/crowdAnim/Blueprints/fishCrowd/worker.fishTargetArray` (`self.assignedWorker`))
    (if (!= _array_index (`self.fishIndex`))
      (bind _output (`self.Check Overlap` _array_element inputVec))
      (if _output
        (return true))))
  (return false))

(fn `Generate Ellipsoid`
  (params (ellipsoidScale :type "Vector Structure") (radius :type "Float (double-precision)") (center :type "Vector Structure") (ellipRotation :type "Rotator Structure"))
  (returns (output :type "Vector Structure"))
  (bind _returnvalue (`KismetMathLibrary.GetPI`))
  (bind _returnvalue_2 (`KismetMathLibrary.RandomFloatInRange` 0.0 _returnvalue))
  (bind _returnvalue_3 (`KismetMathLibrary.RandomFloatInRange` (* radius 0.0) radius))
  (bind _returnvalue_4 (`KismetMathLibrary.RandomFloatInRange` 0.0 (* _returnvalue 2.0)))
  (bind _returnvalue_5 (`KismetMathLibrary.Sin` _returnvalue_2))
  (return (+ center (`KismetMathLibrary.GreaterGreater_VectorRotator` (* ellipsoidScale (`KismetMathLibrary.MakeVector` (* _returnvalue_5 (`KismetMathLibrary.Cos` _returnvalue_4) _returnvalue_3) (* _returnvalue_3 _returnvalue_5 (`KismetMathLibrary.Sin` _returnvalue_4)) (* (`KismetMathLibrary.Cos` _returnvalue_2) _returnvalue_3))) ellipRotation))))

(fn `generateCleanEllipsoid`
  (params (ellipsoidScale :type "Vector Structure") (center :type "Vector Structure") (radius :type "Float (double-precision)") (ellipRotation :type "Rotator Structure"))
  (returns (outputVec :type "Vector Structure"))
  (locals (overLap :type Boolean :default true) (loopNum :type Integer) (generatedVec :type "Vector Structure"))
  (bind _generatedvec (`local.generatedVec`))
  (while (and (`local.overLap`) (<= (`local.loopNum`) (`/Game/crowdAnim/Blueprints/fishCrowd/fishSchool.loopmax` (`self.schoolParent`))))
    (bind _output (`self.Generate Ellipsoid` ellipsoidScale radius center ellipRotation))
    (bind _output_2 (`self.checkOverlapWithOthers` _output))
    (set `local.overLap` _output_2)
    (set `local.generatedVec` _output)
    (set `local.loopNum` (+ (`local.loopNum`) 1)))
  (`KismetArrayLibrary.Array_Set` (`/Game/crowdAnim/Blueprints/fishCrowd/worker.fishTargetArray` (`self.assignedWorker`)) (`self.fishIndex`) _generatedvec)
  (return _generatedvec))

(fn `rotateFish`
  (params (deltaSecond :type "Float (double-precision)"))
  (`self.K2_SetActorRotation` (`KismetMathLibrary.RLerp` (`self.K2_GetActorRotation`) (`self.rotation`) (* deltaSecond (`self.turnSpeed`)) true)))

(fn `Set Mesh Rotation`
  (`SceneComponent.K2_SetRelativeRotation` (`self.MeshComponent`) (`self.meshRotation`) false false))

(fn `setMeshScale`
  (`SceneComponent.SetWorldScale3D` (`self.MeshComponent`) (`KismetMathLibrary.Conv_DoubleToVector` (`KismetMathLibrary.RandomFloatInRange` (`self.minScale`) (`self.maxScale`)))))

(fn `swimTo`
  (params (target :type "Vector Structure"))
  (returns (output :type "Vector Structure"))
  (locals (steer :type "Vector Structure"))
  (bind _returnvalue (`self.GetVelocity`))
  (bind _returnvalue_2 (+ (- target (`self.K2_GetActorLocation`)) _returnvalue))
  (if (or (`KismetMathLibrary.Vector_IsZero` _returnvalue_2) (`KismetMathLibrary.Vector_IsNAN` _returnvalue_2))
    (return _returnvalue)
    (else
      (bind _output_get (set `local.steer` _returnvalue_2))
      (return _output_get))))

(fn `swimToBaits`
  (returns (steer :type "Vector Structure"))
  (if (>= (`self.shapeIndex`) (- (`KismetArrayLibrary.Array_Length` (`self.shapeList`)) 0))
    (set `self.shapeIndex` 0))
  (if (>= (`self.baitIndex`) (- (`KismetArrayLibrary.Array_Length` (`self.baitList`)) 0))
    (set `self.baitIndex` 0))
  (bind _output (`self.swimToOneBait`))
  (return _output))

(fn `swimToOneBait`
  (returns (output :type "Vector Structure"))
  (locals (steer :type "Vector Structure") (addOn :type "Vector Structure"))
  (bind _returnvalue (`self.GetVelocity`))
  (bind (_output_x _output_y _output_z _output_w) (`KismetMathLibrary.BreakVector4` (`|GetArrayItem` (`self.shapeList`) (`self.shapeIndex`))))
  (bind _asbait (cast `/Game/crowdAnim/Blueprints/fishCrowd/bait` (`|GetArrayItem` (`self.baitList`) (`self.baitIndex`))))
  (bind _returnvalue_2 (- (+ (`self.K2_GetActorLocation` _asbait) (`self.addOn_global`)) (`self.K2_GetActorLocation`)))
  (bind _returnvalue_3 (+ _returnvalue_2 _returnvalue))
  (if (or (`KismetMathLibrary.Vector_IsZero` _returnvalue_3) (`KismetMathLibrary.Vector_IsNAN` _returnvalue_3))
    (return _returnvalue)
    (else
      (if (<= (`KismetMathLibrary.VSize` _returnvalue_2) (`self.acceptingRadius`))
        (if (not (== _output_w -1.0))
          (bind _outputvec (`self.generateCleanEllipsoid` (`KismetMathLibrary.MakeVector` _output_x _output_y _output_z) (0.0 0.0 0.0) _output_w (`self.K2_GetActorRotation` _asbait)))
          (set `self.addOn_global` _outputvec))
        (set `self.baitIndex` (+ (`self.baitIndex`) 1))
        (set `self.shapeIndex` (+ (`self.shapeIndex`) 1)))
      (set `local.steer` _returnvalue_3)
      (return (`local.steer`)))))

(fn `UserConstructionScript`)